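; Camera pawn for the Tetris game that places itself to suit the size of the play grid.
; On BeginPlay it reads GridDimensions from BP_TetrisGameMode, doing nothing if the cast fails.
; It then teleports to a fixed rotation, with distance and height scaled from grid height plus padding and lateral offset scaled from grid width.
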(event `self.ReceiveBeginPlay`
  (bind _asbp_tetris_game_mode (cast `/Game/Blueprints/BP_TetrisGameMode` (`GameplayStatics.GetGameMode`)))
  (bind _output_get (set `self.Dimensions` (`TetrisGameMode.gridDimensions` _asbp_tetris_game_mode)))
  (bind _returnvalue (* (+ (`.Y` (break `IntPoint` _output_get)) 5) 50))
  (`self.K2_SetActorLocationAndRotation` (`KismetMathLibrary.MakeVector` (`KismetMathLibrary.Conv_IntToDouble` (+ _returnvalue 1100)) (`KismetMathLibrary.Conv_IntToDouble` (* (break `IntPoint` _output_get) -50)) (`KismetMathLibrary.Conv_IntToDouble` _returnvalue)) (struct :`Yaw` 180.0) false true))

(fn `UserConstructionScript`)