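; BP_GridBorder builds the frame around a vertical grid in the YZ plane, sized by its Width and Height variables.
; On BeginPlay it moves and stretches the Left, Right and Down components into walls and a floor, assuming 100-unit cells.
; A thin Line marks the Height level, with the side walls scaled taller than the grid.
; Placement uses world coordinates, so the frame ignores where the actor is placed.
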(event `self.ReceiveBeginPlay`
  (bind _left (`self.Left`))
  (bind _right (`self.Right`))
  (bind _line (`self.Line`))
  (bind _down (`self.Down`))
  (bind _returnvalue (`KismetMathLibrary.Conv_IntToDouble` (+ (`self.Width`) 2)))
  (bind _returnvalue_2 (`KismetMathLibrary.Conv_IntToDouble` (+ (`self.Height`) 5)))
  (`|ExecutionSequence`
    (:`then_0`
      (`SceneComponent.K2_SetWorldLocation` _left (0.0 100.0 0.0) false true)
      (`SceneComponent.SetRelativeScale3D` _left (`KismetMathLibrary.MakeVector` 1.0 1.0 _returnvalue_2)))
    (:`then_1`
      (`SceneComponent.K2_SetWorldLocation` _right (`KismetMathLibrary.MakeVector` 0.0 (`KismetMathLibrary.Conv_IntToDouble` (* (`self.Width`) -100))) false true)
      (`SceneComponent.SetRelativeScale3D` _right (`KismetMathLibrary.MakeVector` 1.0 1.0 _returnvalue_2)))
    (:`then_2`
      (`SceneComponent.K2_SetWorldLocation` _down (0.0 100.0 -100.0) false true)
      (`SceneComponent.SetRelativeScale3D` _down (`KismetMathLibrary.MakeVector` 1.0 _returnvalue 1.0)))
    (:`then_3`
      (`SceneComponent.K2_SetWorldLocation` _line (`KismetMathLibrary.MakeVector` 0.0 100.0 (`KismetMathLibrary.Conv_IntToDouble` (* (`self.Height`) 100))) false true)
      (`SceneComponent.SetRelativeScale3D` _line (`KismetMathLibrary.MakeVector` 1.0 _returnvalue 0.05)))))

(fn `UserConstructionScript`)