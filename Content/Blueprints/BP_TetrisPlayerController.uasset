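; Tetris player controller that routes player input to the Board and manages the score, start and game-over widgets.
; SetController stores the Board, creates the widgets and binds the score HUD to TetrisGameState score and multiplier change events.
; Enhanced Input mapping contexts separate the start screen from play: starting calls the game mode and enables move, rotate and speed-up controls.
; Game-over and restart events toggle widget visibility and mouse capture.
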(event `SetController`
  (params (Board :type "Board Object Reference"))
  (set `self.Board` Board)
  (`EnhancedInputSubsystemInterface.AddMappingContext` (subsystem `EnhancedInputLocalPlayerSubsystem`) "/Game/Blueprints/Controls/IM_StarGame.IM_StarGame" 0 (struct))
  (bind _astetris_game_state (cast `TetrisGameState` (`GameplayStatics.GetGameState`)))
  (bind _returnvalue (`|CreateWidget` "/Game/Blueprints/UI/W_Score.W_Score_C" self))
  (`UserWidget.AddToViewport` _returnvalue 0)
  (`|ExecutionSequence`
    (:`then_0`
      (add `TetrisGameState.OnMultChanged` _astetris_game_state (delegate `Change mult`)))
    (:`then_1`
      (add `TetrisGameState.OnScoreChanged` _astetris_game_state (delegate `Cange score`))
      (bind _returnvalue_2 (`|CreateWidget` "/Game/Blueprints/UI/W_StartGame.W_StartGame_C" self))
      (bind _output_get (set `self.StartGameWidget` _returnvalue_2))
      (`UserWidget.AddToViewport` _output_get 0)
      (bind _returnvalue_3 (`|CreateWidget` "/Game/Blueprints/UI/W_GameOver.W_GameOver_C" self))
      (bind _output_get_2 (set `self.GameOverWidget` _returnvalue_3))
      (`UserWidget.AddToViewport` _output_get_2 0))))

(event `Change mult`
  (params (mult :type Integer))
  (`ScoreWidget.SetMultiplier` (stale `SetController` _returnvalue) mult))

(event `Cange score`
  (params (score :type Integer))
  (`ScoreWidget.SetScore` (stale `SetController` _returnvalue) score))

(event `OnGameOver`
  (bind _gameoverwidget (`self.GameOverWidget`))
  (bind _astetris_game_state (cast `TetrisGameState` (`GameplayStatics.GetGameState`)))
  (`/Game/Blueprints/UI/W_GameOver.SetScore` _gameoverwidget (`TetrisGameState.score` _astetris_game_state))
  (set `Widget.Visibility` "Visible" _gameoverwidget)
  (set `self.bShowMouseCursor` true)
  (`GameplayStatics.SetViewportMouseCaptureMode` "NoCapture"))

(event `RestartGame`
  (`EnhancedInputSubsystemInterface.AddMappingContext` (subsystem `EnhancedInputLocalPlayerSubsystem`) "/Game/Blueprints/Controls/IM_StarGame.IM_StarGame" 0 (struct))
  (set `Widget.Visibility` "Visible" (`self.StartGameWidget`))
  (set `self.bShowMouseCursor` false)
  (`GameplayStatics.SetViewportMouseCaptureMode` "CapturePermanently_IncludingInitialMouseDown"))

(event `EnhancedInput|/Game/Blueprints/Controls/IA_MovePiece`
  (params (ActionValue :type "Float (double-precision)") (ElapsedSeconds :type "Float (double-precision)") (TriggeredSeconds :type "Float (double-precision)") (InputAction :type "InputAction Object Reference" :default "/Game/Blueprints/Controls/IA_MovePiece.IA_MovePiece"))
  (:`Triggered`
    (`Board.MoveBlock` (`self.Board`) ActionValue)))

(event `EnhancedInput|/Game/Blueprints/Controls/IA_Rotate`
  (params (ActionValue :type "Float (double-precision)") (ElapsedSeconds :type "Float (double-precision)") (TriggeredSeconds :type "Float (double-precision)") (InputAction :type "InputAction Object Reference" :default "/Game/Blueprints/Controls/IA_Rotate.IA_Rotate"))
  (:`Started`
    (`Board.RotateBlock` (`self.Board`) ActionValue)))

(event `EnhancedInput|/Game/Blueprints/Controls/IA_SpeedUp`
  (params (ActionValue :type "Float (double-precision)") (ElapsedSeconds :type "Float (double-precision)") (TriggeredSeconds :type "Float (double-precision)") (InputAction :type "InputAction Object Reference" :default "/Game/Blueprints/Controls/IA_SpeedUp.IA_SpeedUp"))
  (bind _board (`self.Board`))
  (:`Started`
    (`Board.setFastSpeed` _board))
  (:`Completed`
    (`Board.setSlowSpeed` _board)))

(event `Allow Tetris Inputs`
  (`EnhancedInputSubsystemInterface.AddMappingContext` (subsystem `EnhancedInputLocalPlayerSubsystem`) "/Game/Blueprints/Controls/IM_TetrisInput.IM_TetrisInput" 0 (struct)))

(event `Deny Tetris Imputs`
  (`EnhancedInputSubsystemInterface.RemoveMappingContext` (subsystem `EnhancedInputLocalPlayerSubsystem`) "/Game/Blueprints/Controls/IM_TetrisInput.IM_TetrisInput" (struct)))

(event `EnhancedInput|/Game/Blueprints/Controls/IA_StartGame`
  (params (ActionValue :type Boolean) (ElapsedSeconds :type "Float (double-precision)") (TriggeredSeconds :type "Float (double-precision)") (InputAction :type "InputAction Object Reference" :default "/Game/Blueprints/Controls/IA_StartGame.IA_StartGame"))
  (:`Triggered`
    (`EnhancedInputSubsystemInterface.RemoveMappingContext` (subsystem `EnhancedInputLocalPlayerSubsystem`) "/Game/Blueprints/Controls/IM_StarGame.IM_StarGame" (struct))
    (set `Widget.Visibility` "Hidden" (`self.StartGameWidget`))
    (bind _asbp_tetris_game_mode (cast `/Game/Blueprints/BP_TetrisGameMode` (`GameplayStatics.GetGameMode`)))
    (`TetrisGameMode.StartGame` _asbp_tetris_game_mode)
    (`self.Allow Tetris Inputs`)))

(fn `UserConstructionScript`)