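; Game mode Blueprint for a Tetris game that sets up the player controller and playfield border and handles losing.
; On BeginPlay it casts player 0's controller, hands it the Board reference and initializes it, then spawns a BP_GridBorder sized from GridDimensions.
; LoseGame disables Tetris input on that controller and prints a long-lasting game-ended message.
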(event `self.ReceiveBeginPlay`
  (bind (_griddimensions_x _griddimensions_y) (break `IntPoint` (`self.gridDimensions`)))
  (`parent.ReceiveBeginPlay`)
  (bind _asbp_tetris_player_controller (cast `/Game/Blueprints/BP_TetrisPlayerController` (`GameplayStatics.GetPlayerController` 0)))
  (bind _output_get (set `self.Controller` _asbp_tetris_player_controller))
  (set `/Game/Blueprints/BP_TetrisPlayerController.Board` (`self.board`) _output_get)
  (`/Game/Blueprints/BP_TetrisPlayerController.SetController` _output_get)
  (`|SpawnActorFromClass` "/Game/Blueprints/BP_GridBorder.BP_GridBorder_C" (`KismetMathLibrary.MakeTransform` (0.0 100.0 -100.0)) "Undefined" "MultiplyWithRoot" null _griddimensions_x _griddimensions_y null)
  (`KismetSystemLibrary.LogString` "Setted-----------------------------------------------------------------------------"))

(event `self.LoseGame`
  (`/Game/Blueprints/BP_TetrisPlayerController.Deny Tetris Imputs` (`self.Controller`))
  (`KismetSystemLibrary.PrintText` "Game Ended" true true (struct :`R` 0.120279 :`G` 1.0 :`B` 0.027887 :`A` 1.0) 1002.0))

(fn `UserConstructionScript`)